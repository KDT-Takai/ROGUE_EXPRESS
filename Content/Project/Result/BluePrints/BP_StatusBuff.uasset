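; BP_StatusBuff converts a status-up skill card into an SPlayerStatus struct representing a player stat buff.
; UseStatusUp switches on the card's ID and calls a function named after that ID, covering health, attack, attack speed and fuel.
; Each function puts the card's Amount into its stat, with health and fuel setting both maximum and current values.
; It only returns the struct; the event graph is empty.
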(event EventBeginPlay)

(event Collision|EventActorBeginOverlap
  (params (OtherActor :type Actor%20Object%20Reference)))

(event EventTick
  (params (DeltaSeconds :type Float%20%28single-precision%29)))

(fn ConstructionScript)

(fn UseStatusUp
  (params (SkillCardData :type ST%20Skill%20Card%20Data%20Structure))
  (switch int (.ID (Utilities|Struct|BreakST_SkillCardData SkillCardData))
    (:301
      (bind _status (CallFunction|301 SkillCardData))
      (return _status))
    (:302
      (bind _status_2 (CallFunction|302 SkillCardData))
      (return _status_2))
    (:303
      (bind _status_3 (CallFunction|303 SkillCardData))
      (return _status_3))
    (:304
      (bind _status_4 (CallFunction|304 SkillCardData))
      (return _status_4))))

(fn 301
  (params (skilldata :type ST%20Skill%20Card%20Data%20Structure))
  (bind _amount (Utilities|Struct|BreakST_SkillCardData skilldata))
  (return (Utilities|Struct|MakeS_PlayerStatus _amount _amount)))

(fn 302
  (params (skilldata :type ST%20Skill%20Card%20Data%20Structure))
  (return (Utilities|Struct|MakeS_PlayerStatus 0.0 0.0 0.0 0.0 (.Amount (Utilities|Struct|BreakST_SkillCardData skilldata)))))

(fn 303
  (params (skilldata :type ST%20Skill%20Card%20Data%20Structure))
  (return (Utilities|Struct|MakeS_PlayerStatus 0.0 0.0 0.0 0.0 0.0 (.Amount (Utilities|Struct|BreakST_SkillCardData skilldata)))))

(fn 304
  (params (skilldata :type ST%20Skill%20Card%20Data%20Structure))
  (bind _amount (Utilities|Struct|BreakST_SkillCardData skilldata))
  (return (Utilities|Struct|MakeS_PlayerStatus 0.0 0.0 _amount _amount)))