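; BP_Takarabako is a result-side actor that presents treasure chest card selection to the player.
; On BeginPlay it creates the WBP_Takarabako widget, adds it to the viewport and runs CheckChest.
; CheckChest reads PlayerStatus.ChestCount from BP_GameInstance and, if it is nonzero, shows the selectable cards and locks input to the widget in UI-only mode.
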(event EventBeginPlay
  ;[0.15 0.15 0.15 0.5] ビューポート初期化
  (bind _returnvalue (UserInterface|CreateWidget "/Game/Project/Result/BluePrints/WBP_Takarabako.WBP_Takarabako_C"))
  (UserInterface|Viewport|AddtoViewport _returnvalue 0)
  (Variables|Default|SetW_takarabako _returnvalue)
  (CallFunction|CheckChest))

(event Collision|EventActorBeginOverlap
  (params (OtherActor :type Actor%20Object%20Reference)))

(event EventTick
  (params (DeltaSeconds :type Float%20%28single-precision%29)))

(fn ConstructionScript)

(fn CheckChest
  (bind _w_takarabako (Variables|Default|GetW_takarabako))
  ;[0.15 0.15 0.15 0.5] 宝箱があるかの確認
  (bind _asbp_game_instance (Utilities|Casting|CastToBP_GameInstance (Game|GetGameInstance)))
  (if (!= (.ChestCount (Utilities|Struct|BreakS_PlayerStatus (Variables|/Game/Project/System/BP_GameInstance.BP_GameInstance_C|GetPlayerStatus _asbp_game_instance))) 0.0)
    ;[0.15 0.15 0.15 0.5] カードの表示
    (Default|ShowSelectCards _w_takarabako)
    (Input|SetInputModeUIOnly 0 _w_takarabako "LockAlways" false)
    (else
      (return))))