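; BP_OpenLevel is a Blueprint that manages the result screen widget, WBP_Result.
; On BeginPlay it creates and stores the widget, adds it to the viewport, sets UI-only input focused on it, then hides it.
; The ResultView event later makes the stored widget visible.
; Despite its name, its graph contains no level-opening logic.
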(event Custom|ResultView
  (Widget|SetVisibility (Variables|Default|GetResultWi) "Visible"))

(event EventBeginPlay
  (bind _returnvalue (UserInterface|CreateWidget "/Game/Project/Result/BluePrints/WBP_Result.WBP_Result_C"))
  (Variables|Default|SetResultWi _returnvalue)
  (UserInterface|Viewport|AddtoViewport _returnvalue 0)
  (Input|SetInputModeUIOnly (Game|GetPlayerController 0) _returnvalue "DoNotLock" false)
  (Widget|SetVisibility _returnvalue "Hidden"))

(fn ConstructionScript)