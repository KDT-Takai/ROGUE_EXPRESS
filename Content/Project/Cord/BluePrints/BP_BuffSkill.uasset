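; BP_BuffSkill turns buff skill cards into player status changes: emergency repair, refuelling, drain and attack speed.
; UseBuff plays a sound, then dispatches on card ID to a skill function returning a status delta.
; Drain and attack-speed skills set named timers for Limit functions, marked unfinished.
; These re-find the card in SkillCardDataTable and pass the negated amount to BP_FirstPersonCharacter's Buff.
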(fn ConstructionScript)

(fn UseBuff
  (params (SkillCardData :type ST%20Skill%20Card%20Data%20Structure))
  (Audio|PlaySound2D "/Game/Project/Player/Assets/SE/MagecSE.MagecSE" 1.0 1.0 0.0 0 0)
  (switch int (.ID (Utilities|Struct|BreakST_SkillCardData SkillCardData))
    (:101
      (bind _status (CallFunction|Skill:101 SkillCardData))
      (return _status))
    (:102
      (bind _status_2 (CallFunction|Skill:102 SkillCardData))
      (return _status_2))
    (:103
      (bind _status_3 (CallFunction|Skill:103 SkillCardData))
      (return _status_3))
    (:104
      (bind _status_4 (CallFunction|Skill:104 SkillCardData))
      (return _status_4))))

(fn Skill:101
  (params (SkillData :type ST%20Skill%20Card%20Data%20Structure))
  ;[0.15 0.15 0.15 0.5] 緊急修理
  (return (Utilities|Struct|MakeS_PlayerStatus 0.0 (.Amount (Utilities|Struct|BreakST_SkillCardData SkillData)))))

(fn Skill:102
  (params (SkillData :type ST%20Skill%20Card%20Data%20Structure))
  ;[0.15 0.15 0.15 0.5] 燃料補給
  (return (Utilities|Struct|MakeS_PlayerStatus 0.0 0.0 0.0 (.Amount (Utilities|Struct|BreakST_SkillCardData SkillData)))))

(fn Skill:103
  (params (SkillData :type ST%20Skill%20Card%20Data%20Structure))
  (bind (_id _skillname _category _rarity _amount _durationtime) (Utilities|Struct|BreakST_SkillCardData SkillData))
  ;[0.15 0.15 0.15 0.5] 時間経過で元のステータスに戻す処理
  (Utilities|Time|SetTimerbyFunctionName 0 "Skill:103Limit" (Math|Conversions|ToFloat(Integer) _durationtime)) ; バフの値をもとに戻すための関数のセット
  (return (Utilities|Struct|MakeS_PlayerStatus 0.0 0.0 0.0 0.0 0.0 0.0 0.0 0.0 0.0 _amount)))

(fn Skill:104
  (params (SkillData :type ST%20Skill%20Card%20Data%20Structure))
  (bind (_id _skillname _category _rarity _amount _durationtime) (Utilities|Struct|BreakST_SkillCardData SkillData))
  ;[0.15 0.15 0.15 0.5] 時間経過で元のステータスに戻す処理
  (Utilities|Time|SetTimerbyFunctionName 0 "Skill:104Limit" (Math|Conversions|ToFloat(Integer) _durationtime)) ; バフの値をもとに戻すための関数のセット
  (return (Utilities|Struct|MakeS_PlayerStatus 0.0 0.0 0.0 0.0 0.0 _amount)))

(fn Skill:103Limit
  ;[0.15 0.15 0.15 0.5] 作りかけ
  (bind _skillcarddata (CallFunction|GetSKillFroID 103))
  (bind _returnvalue (Actor|GetActorOfClass "/Game/Project/Player/BluePrints/BP_FirstPersonCharacter.BP_FirstPersonCharacter_C"))
  (Default|Buff _returnvalue (Utilities|Struct|MakeS_PlayerStatus 0.0 0.0 0.0 0.0 0.0 0.0 0.0 0.0 0.0 (* (.Amount (Utilities|Struct|BreakST_SkillCardData _skillcarddata)) -1.0)) 0.0)
  (return))

(fn Skill:104Limit
  ;[0.15 0.15 0.15 0.5] 作りかけ
  (bind _skillcarddata (CallFunction|GetSKillFroID 104))
  (bind _returnvalue (Actor|GetActorOfClass "/Game/Project/Player/BluePrints/BP_FirstPersonCharacter.BP_FirstPersonCharacter_C"))
  (Default|Buff _returnvalue (Utilities|Struct|MakeS_PlayerStatus 0.0 0.0 0.0 0.0 0.0 (* (.Amount (Utilities|Struct|BreakST_SkillCardData _skillcarddata)) -1.0)) 0.0)
  (return))

(fn GetSKillFroID
  (params (skillID :type Byte))
  (bind _outrownames (DataTable|GetDataTableRowNames "/Game/Project/Cord/DataTable/SkillCardDataTable.SkillCardDataTable"))
  (for _array_element _outrownames
    (bind _returnvalue (Utilities|GetDataTableRow "/Game/Project/Cord/DataTable/SkillCardDataTable.SkillCardDataTable" _array_element)
      (:then
        (if (== (.ID (Utilities|Struct|BreakST_SkillCardData _returnvalue)) skillID)
          (return _returnvalue))))))