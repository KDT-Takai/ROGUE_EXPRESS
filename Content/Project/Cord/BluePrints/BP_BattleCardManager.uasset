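; Card battle manager actor that runs the player's skill deck across draw, hand, used and unusable piles.
; It loads the deck from the GameInstance or CardFactory, draws randomly with used-pile recycling, and saves it back on EndPlay.
; CardUse pays HP or fuel, triggers attack skills or timed player buffs, then starts a cooldown.
; Unless a card keeps the hand, the whole hand is discarded and redrawn by timer, updating the hand widget.
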(event Custom|CardUse
  (params (Index :type Integer) (WB_Hand :type WB%20Hand%20Object%20Reference))
  (bind _returnvalue (- Index 1))
  (bind _farstpersoncharacter (Variables|Default|GetfarstPersonCharacter))
  (bind _handcards (Variables|Default|GetHandCards))
  (bind _output (Utilities|Array|Get(acopy) _handcards _returnvalue))
  (bind (_id _skillname _category _rarity _amount _durationtime _resourcetype _resourceamount _iskeephand) (Utilities|Struct|BreakST_SkillCardData _output))
  ;[0.15 0.15 0.15 0.5] カードの使用
  (if (Variables|Default|GetCanUse) ; カードを使える状態か判定（CTなどを含む）
    ;;[0.15 0.15 0.15 0.5] ステータス消費確認＆消費
    (bind _resourcenothing (CallFunction|ResourceUse _output))
    (if _resourcenothing
      (switch int (Math|Conversions|ToInteger(Byte) _category)
        (:0
          (Audio|PlaySound2D "/Game/Project/Player/Assets/SE/maou_se_system45.maou_se_system45" 1.0 1.0 0.0 0 0)
          ;;[0.15 0.15 0.15 0.5] 攻撃スキル
          (Default|UseSkill (Variables|Default|GetAttackSkills) _id))
        (:1
          ;[0.15 0.15 0.15 0.5] バフスキル
          (bind _returnstatus (Default|UseBuff (Variables|Default|GetBuffSkill) _output)) ; バフのIDからバフ量の数値を\nステータスの形で取得
          (Default|Buff _farstpersoncharacter _returnstatus 0.0) ; バフの値反映
          (Utilities|Time|SetTimerbyFunctionName _farstpersoncharacter "BuffLimit" (Math|Conversions|ToFloat(Integer) _durationtime)) ; バフの値をもとに戻すための関数のセット
        ))
      ;;[0.15 0.15 0.15 0.5] クールタイム関係
      (Variables|Default|SetCanUse false) ; 使用できない状態へ（ＣＴへ）
      (Utilities|Time|SetTimerbyFunctionName 0 "CoolReset" 1.0)
      (if _iskeephand ; 手札をキープするか
        ;[0.15 0.15 0.15 0.5] 演出つくろうね
        ;;[0.15 0.15 0.15 0.5] 手札をキープして使用済みだけ
        ;; 墓地に送る処理
        (CallFunction|CardtoUsed _output)
        (if (== (Utilities|Array|Length (Variables|Default|GetHandCards)) 0)
          (CallFunction|DrawCard))
        (Default|RefreshUI WB_Hand (Variables|Default|GetHandCards))
        (else
          (CallFunction|HandtoUsed)
          (Default|ProductUseCard (Variables|Default|GetWBHand) _returnvalue)
          (Utilities|Time|SetTimerbyFunctionName 0 "NextHand" 0.8))))))

(event Custom|begin
  (bind _deckcards (Variables|Default|GetDeckCards))
  ;[0.15 0.15 0.15 0.5] ごり押し順番制御
  ;[0.15 0.15 0.15 0.5] CardFactory取得
  (bind _returnvalue (Actor|GetActorOfClass "/Game/Project/Cord/BluePrints/BP_CardFactory.BP_CardFactory_C"))
  (bind _output_get (Variables|Default|SetCardFactory _returnvalue))
  ;[0.15 0.15 0.15 0.5] AttackSkillへの参照取得
  (bind _returnvalue_2 (Actor|GetActorOfClass "/Game/Project/Player/BluePrints/BP_AttackSkill.BP_AttackSkill_C"))
  (Variables|Default|SetAttackSkills _returnvalue_2)
  ;[0.15 0.15 0.15 0.5] バフスキルへの参照
  (bind _returnvalue_3 (Actor|GetActorOfClass "/Game/Project/Cord/BluePrints/BP_BuffSkill.BP_BuffSkill_C"))
  (Variables|Default|SetBuffSkill _returnvalue_3)
  ;[0.15 0.15 0.15 0.5] プレイヤーへの参照
  (bind _returnvalue_4 (Actor|GetActorOfClass "/Game/Project/Player/BluePrints/BP_FirstPersonCharacter.BP_FirstPersonCharacter_C"))
  (Variables|Default|SetfarstPersonCharacter _returnvalue_4)
  ;[0.15 0.15 0.15 0.5] ゲームインスタンスからカード取得
  (bind _asbp_game_instance (Utilities|Casting|CastToBP_GameInstance (Game|GetGameInstance)))
  (if (Utilities|Array|IsEmpty (Variables|/Game/Project/System/BP_GameInstance.BP_GameInstance_C|GetDeck _asbp_game_instance)) ; 空なら初期デッキ制作
    ;[0.15 0.15 0.15 0.5] 初期デッキ制作
    (bind _startdeck (Default|CreateStartDeck _output_get))
    (Utilities|Array|AppendArray _deckcards _startdeck)
    (else
      (Utilities|Array|AppendArray _deckcards (Variables|/Game/Project/System/BP_GameInstance.BP_GameInstance_C|GetDeck _asbp_game_instance))
      (Utilities|Array|Clear (Variables|/Game/Project/System/BP_GameInstance.BP_GameInstance_C|GetDeck _asbp_game_instance))))
  (CallFunction|DrawCard) ; 手札のドロー
  ;[0.15 0.15 0.15 0.5] SysPownの持つ処理を実行のため一時的に取得
  (bind _returnvalue_5 (Actor|GetActorOfClass "/Game/Project/Cord/BluePrints/BP_CardSysPown.BP_CardSysPown_C"))
  (Variables|Default|SetWBHand (Variables|/Game/Project/Cord/BluePrints/BP_CardSysPown.BP_CardSysPown_C|GetWBHandUI _returnvalue_5))
  (Default|RefreshUI (Variables|/Game/Project/Cord/BluePrints/BP_CardSysPown.BP_CardSysPown_C|GetWBHandUI _returnvalue_5) (Variables|Default|GetHandCards)) ; UIの更新
  (Default|ProductFarstDrow (Variables|/Game/Project/Cord/BluePrints/BP_CardSysPown.BP_CardSysPown_C|GetWBHandUI _returnvalue_5)))

(event Custom|SaveCards
  ;[0.15 0.15 0.15 0.5] ゲームインスタンスにカードを保存
  (CallFunction|AllCardstoDeck)
  (bind _asbp_game_instance (Utilities|Casting|CastToBP_GameInstance (Game|GetGameInstance)))
  (for _array_element (Variables|Default|GetDeckCards)
    (Utilities|Array|Add (Variables|/Game/Project/System/BP_GameInstance.BP_GameInstance_C|GetDeck _asbp_game_instance) _array_element)))

(event EventBeginPlay
  ;[0.15 0.15 0.15 0.5] ごり押し順番制御
)

(event EventEndPlay
  (params (EndPlayReason :type EEndPlayReason%20Enum :default "Destroyed"))
  ;[0.15 0.15 0.15 0.5] ゲームインスタンスにカードを保存
  (CallFunction|AllCardstoDeck)
  (bind _asbp_game_instance (Utilities|Casting|CastToBP_GameInstance (Game|GetGameInstance)))
  (for _array_element (Variables|Default|GetDeckCards)
    (Utilities|Array|Add (Variables|/Game/Project/System/BP_GameInstance.BP_GameInstance_C|GetDeck _asbp_game_instance) _array_element)))

(fn ConstructionScript)

(fn DeckReset
  (bind _usedcards (Variables|Default|GetUsedCards))
  (Utilities|Array|AppendArray (Variables|Default|GetDeckCards) _usedcards)
  (Utilities|Array|Clear _usedcards))

(fn MovetoCantUseCards
  (params (index :type Integer))
  (Utilities|Array|Add (Variables|Default|GetCantUseCards) (Utilities|Array|Get(acopy) (Variables|Default|GetHandCards) index))
  (Utilities|Array|RemoveIndex (Variables|Default|GetHandCards) index))

(fn HandtoUsed
  (bind _handcards (Variables|Default|GetHandCards))
  (Utilities|Array|AppendArray (Variables|Default|GetUsedCards) _handcards)
  (Utilities|Array|Clear _handcards))

(fn AllCardstoDeck
  (bind _deckcards (Variables|Default|GetDeckCards))
  (bind _handcards (Variables|Default|GetHandCards))
  (bind _usedcards (Variables|Default|GetUsedCards))
  (bind _cantusecards (Variables|Default|GetCantUseCards))
  (Utilities|Array|AppendArray _deckcards _handcards)
  (Utilities|Array|Clear _handcards)
  (Utilities|Array|AppendArray _deckcards _usedcards)
  (Utilities|Array|Clear _usedcards)
  (Utilities|Array|AppendArray _deckcards _cantusecards)
  (Utilities|Array|Clear _cantusecards))

(fn DrawCard
  (bind _deckcards (Variables|Default|GetDeckCards))
  (for _index (range 0 2)
    ;[0.15 0.15 0.15 0.5] カードをドローする　山札がなければ墓地から山に戻して引く
    (if (!= (Utilities|Array|Length (Variables|Default|GetDeckCards)) 0)
      _
      (else
        (CallFunction|DeckReset)))
    (bind _returnvalue (Utilities|Array|Length (Variables|Default|GetDeckCards)))
    (bind _returnvalue_2 (Math|Random|RandomIntegerinRange 0 (- _returnvalue 1)))
    (Utilities|Array|Add (Variables|Default|GetHandCards) (Utilities|Array|Get(acopy) _deckcards _returnvalue_2))
    (Utilities|Array|RemoveIndex _deckcards _returnvalue_2)))

(fn AddtoDeck
  (params (Skill :type ST%20Skill%20Card%20Data%20Structure))
  (Utilities|Array|Add (Variables|Default|GetDeckCards) Skill))

(fn CoolReset
  (Variables|Default|SetCanUse true))

(fn CardtoUsed
  (params (usedCard :type ST%20Skill%20Card%20Data%20Structure))
  (Utilities|Array|Add (Variables|Default|GetUsedCards) usedCard)
  (Utilities|Array|RemoveItem (Variables|Default|GetHandCards) usedCard))

(fn ResourceUse
  (params (skilldata :type ST%20Skill%20Card%20Data%20Structure))
  (bind (_id _skillname _category _rarity _amount _durationtime _resourcetype _resourceamount) (Utilities|Struct|BreakST_SkillCardData skilldata))
  (bind _farstpersoncharacter (Variables|Default|GetfarstPersonCharacter))
  (bind _playerstatus (Variables|/Game/Project/Player/BluePrints/BP_FirstPersonCharacter.BP_FirstPersonCharacter_C|GetPlayerStatus _farstpersoncharacter))
  (bind (_maxhp _hp _maxfuel _fuel) (Utilities|Struct|BreakS_PlayerStatus _playerstatus))
  (switch int (Math|Conversions|ToInteger(Byte) _resourcetype)
    (:1
      (if (< _resourceamount _hp)
        (Default|TakeDamage _farstpersoncharacter (Math|Conversions|ToFloat(Integer) _resourceamount))
        (return true)
        (else
          _)))
    (:2
      (if (< _resourceamount _fuel)
        (Default|UseFuel _farstpersoncharacter (Math|Conversions|ToFloat(Integer) _resourceamount))
        (return true)
        (else
          _))))
  (return false))

(fn NextHand
  (CallFunction|DrawCard)
  (Default|RefreshUI (Variables|Default|GetWBHand) (Variables|Default|GetHandCards)))