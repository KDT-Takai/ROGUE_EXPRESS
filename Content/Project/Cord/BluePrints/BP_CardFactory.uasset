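; BP_CardFactory builds skill card data and the starting deck for card battles.
; CreateStartDeck turns each ID in StartDeckDataIDs into card data via CreateCardData, appends it to DeckData and returns that array.
; Lookup is a linear scan of SkillCardDataTable rows, matching on the ID field rather than the row name.
; A custom Begin event, used instead of BeginPlay to control initialization order, caches the BP_BattleCardManager reference.
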(event Custom|Begin
  ;[0.15 0.15 0.15 0.5] ごり押し順番制御
  (bind _returnvalue (Actor|GetActorOfClass "/Game/Project/Cord/BluePrints/BP_BattleCardManager.BP_BattleCardManager_C")) ; BattleCardManagerの参照を取得
  (Variables|Default|SetBattleCardManager _returnvalue))

(event EventBeginPlay
  ;[0.15 0.15 0.15 0.5] ごり押し順番制御
)

(event Collision|EventActorBeginOverlap
  (params (OtherActor :type Actor%20Object%20Reference)))

(event EventTick
  (params (DeltaSeconds :type Float%20%28single-precision%29)))

(fn ConstructionScript)

(fn CreateCardData
  (params (CreateID :type Byte))
  ;[0.15 0.15 0.15 0.5] カードの生成処理
  (bind _skillcarddata (CallFunction|CheckCreateID CreateID))
  (return _skillcarddata))

(fn CreateStartDeck
  (bind _deckdata (LocalVariables|GetDeckData))
  ;[0.15 0.15 0.15 0.5] 指定のカードをすべて作成
  (for _array_element (Variables|Default|GetStartDeckDataIDs)
    (bind _carddata (CallFunction|CreateCardData _array_element))
    (Utilities|Array|Add _deckdata _carddata))
  (return _deckdata) ; 作成されたデッキデータを返す
)

(fn CheckCreateID
  (params (skillID :type Byte))
  (bind _outrownames (DataTable|GetDataTableRowNames "/Game/Project/Cord/DataTable/SkillCardDataTable.SkillCardDataTable"))
  (for _array_element _outrownames
    (bind _returnvalue (Utilities|GetDataTableRow "/Game/Project/Cord/DataTable/SkillCardDataTable.SkillCardDataTable" _array_element)
      (:then
        (if (== (.ID (Utilities|Struct|BreakST_SkillCardData _returnvalue)) skillID)
          (return _returnvalue))))))