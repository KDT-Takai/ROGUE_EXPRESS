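; BP_CardSysPown bootstraps the battle card system and relays the player's number input to it.
; On BeginPlay it explicitly calls Begin on BP_CardFactory, creates the WB_Hand widget, sets game-only input, then calls Begin on BP_BattleCardManager, forcing initialization order.
; NumKeysInput passes the index and hand widget to the manager's CardUse, which handles all usability checks.
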(event Custom|NumKeysInput
  (params (InputNum :type Integer))
  (Default|CardUse (Variables|Default|GetBattleCardManager) InputNum (Variables|Default|GetWBHandUI)) ; カードを使用できるかなどの判定はメソッド内で行う\nここはただただ中継
)

(event EventBeginPlay
  ;[0.15 0.15 0.15 0.5] ごり押し順番制御
  (bind _returnvalue (Actor|GetActorOfClass "/Game/Project/Cord/BluePrints/BP_CardFactory.BP_CardFactory_C"))
  (Default|Begin _returnvalue)
  ;[0.15 0.15 0.15 0.5] BattleCardMGの取得
  (bind _returnvalue_2 (Actor|GetActorOfClass "/Game/Project/Cord/BluePrints/BP_BattleCardManager.BP_BattleCardManager_C"))
  (Variables|Default|SetBattleCardManager _returnvalue_2)
  ;[0.15 0.15 0.15 0.5] ビューポートの作成
  (bind _returnvalue_3 (UserInterface|CreateWidget "/Game/Project/Cord/BluePrints/WB_Hand.WB_Hand_C"))
  (bind _output_get (Variables|Default|SetWBHandUI _returnvalue_3))
  (UserInterface|Viewport|AddtoViewport _output_get 0)
  (Input|SetInputModeGameOnly 0 false) ; ビューポート操作設定
  ;[0.15 0.15 0.15 0.5] ごり押し順番制御
  (Default|Begin (Variables|Default|GetBattleCardManager)))

(event Collision|EventActorBeginOverlap
  (params (OtherActor :type Actor%20Object%20Reference)))

(event EventTick
  (params (DeltaSeconds :type Float%20%28single-precision%29)))

(fn ConstructionScript)