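; BP_Target is an enemy target actor that advances along the X axis and damages the player upon reaching their X position.
; Each Tick moves it in negative X at constant speed, without sweep, while the player's X is lower.
; Otherwise it subtracts its EnemyStatus Attack from the BP_FirstPersonCharacter's PlayerStatus HP, prints a message and destroys itself.
; The hit test compares only X, with no collision or overlap check.
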(event EventTick
  (params (DeltaSeconds :type Float%20%28single-precision%29))
  (bind _returnvalue (Game|GetPlayerCharacter 0))
  (if (< (.x (Transformation|GetActorLocation _returnvalue)) (.x (Transformation|GetActorLocation)))
    (Transformation|AddActorWorldOffset (Math|Vector|MakeVector (* DeltaSeconds -3e+02) 0.0 0.0))
    (else
      (bind _asbp_first_person_character (Utilities|Casting|CastToBP_FirstPersonCharacter _returnvalue))
      (Utilities|Struct|SetmembersinS_PlayerStatus (Variables|/Game/FirstPerson/Blueprints/BP_FirstPersonCharacter.BP_FirstPersonCharacter_C|GetPlayerStatus _asbp_first_person_character) (- (.HP (Utilities|Struct|BreakS_PlayerStatus (Variables|/Game/FirstPerson/Blueprints/BP_FirstPersonCharacter.BP_FirstPersonCharacter_C|GetPlayerStatus _asbp_first_person_character))) (.Attack (Utilities|Struct|BreakS_EnemyStatus (Variables|Default|GetEnemyStatus)))))
      (Development|PrintString "Damage")
      (Actor|DestroyActor))))

(fn ConstructionScript)