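; BP_AttackSkill runs the player's attack skills, with UseSkill dispatching a SkillID to Blade, Beam, Mine, Turret or Grenade.
; Blade deals radial damage around the player, while Beam sphere-traces along the camera, both scaling with PlayerStatus.Attack.
; Mine and Turret spawn actors at a camera line-trace hit, and Grenade spawns from the camera.
; UseSkill fires Beam once; the looping-timer StartBeam is never called here.
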(event Custom|Blade
  (bind _returnvalue (Game|GetPlayerCharacter 0))
  (bind _asbp_first_person_character (Utilities|Casting|CastToBP_FirstPersonCharacter _returnvalue))
  (bind _returnvalue_2 (Transformation|GetActorLocation _asbp_first_person_character))
  ;[0.15 0.15 0.15 0.5] ブレード
  (Game|Damage|ApplyRadialDamage (* (.Attack (Utilities|Struct|BreakS_PlayerStatus (Variables|/Game/Project/Player/BluePrints/BP_FirstPersonCharacter.BP_FirstPersonCharacter_C|GetPlayerStatus _asbp_first_person_character))) 3.0) _returnvalue_2 2.2e+03 0 (Utilities|Array|MakeArray _asbp_first_person_character) 0 0 false "ECC_Visibility")
  (Niagara|SpawnSystematLocation "/Game/NiagaraExamples/FX_Misc/NS_Boundary_Cylinder.NS_Boundary_Cylinder" (+ _returnvalue_2 (* (Math|Vector|GetForwardVector (Variables|/Game/Project/Player/BluePrints/BP_FirstPersonCharacter.BP_FirstPersonCharacter_C|GetFirstPersonCamera _asbp_first_person_character)) 1.5e+02)) "0, 0, 0" "35.000000,35.000000,35.000000")
  (Rendering|Debug|DrawDebugSphere _returnvalue_2 2e+03 12 "(R=1.000000,G=0.000000,B=0.000000,A=1.000000)" 1.0))

(event Custom|Beam
  (bind _returnvalue (Game|GetPlayerCharacter 0))
  (bind _asbp_first_person_character (Utilities|Casting|CastToBP_FirstPersonCharacter _returnvalue))
  (bind _firstpersoncamera (Variables|/Game/Project/Player/BluePrints/BP_FirstPersonCharacter.BP_FirstPersonCharacter_C|GetFirstPersonCamera _asbp_first_person_character))
  (bind _returnvalue_2 (Transformation|GetWorldLocation _firstpersoncamera))
  ;[0.15 0.15 0.15 0.5] ビーム
  (bind _outhits (Collision|MultiSphereTraceForObjects _returnvalue_2 (+ _returnvalue_2 (* (Math|Vector|GetForwardVector _firstpersoncamera) 1e+04)) 3e+01 (Utilities|Array|MakeArray "ObjectTypeQuery3" "ObjectTypeQuery2") false (Utilities|Array|MakeArray _asbp_first_person_character) "ForDuration"))
  (for _array_element _outhits
    (Game|Damage|ApplyDamage (.HitActor (Collision|BreakHitResult _array_element)) (* (.Attack (Utilities|Struct|BreakS_PlayerStatus (Variables|/Game/Project/Player/BluePrints/BP_FirstPersonCharacter.BP_FirstPersonCharacter_C|GetPlayerStatus (.AsBP%20First%20Person%20Character (Utilities|Casting|CastToBP_FirstPersonCharacter (Game|GetPlayerCharacter 0)))))) 2.5) 0 0)))

(event Custom|Turret
  (bind _returnvalue (Game|GetPlayerCharacter 0))
  (bind _asbp_first_person_character (Utilities|Casting|CastToBP_FirstPersonCharacter _returnvalue))
  (bind _firstpersoncamera (Variables|/Game/Project/Player/BluePrints/BP_FirstPersonCharacter.BP_FirstPersonCharacter_C|GetFirstPersonCamera _asbp_first_person_character))
  ;[0.15 0.15 0.15 0.5] タレット
  (bind _outhit (Collision|LineTraceByChannel (Transformation|GetWorldLocation _firstpersoncamera) (+ (Transformation|GetWorldLocation _firstpersoncamera) (* (Math|Vector|GetForwardVector _firstpersoncamera) 5e+03)) "TraceTypeQuery1" true 0 "None"))
  (Game|SpawnActorfromClass "/Game/Project/Player/BluePrints/BP_Skill_Turret.BP_Skill_Turret_C" (Math|Transform|MakeTransform (.Location (Collision|BreakHitResult _outhit))) "Undefined" "MultiplyWithRoot" 0 0))

(event Custom|Grenade
  (bind _returnvalue (Game|GetPlayerCharacter 0))
  (bind _asbp_first_person_character (Utilities|Casting|CastToBP_FirstPersonCharacter _returnvalue))
  (bind _firstpersoncamera (Variables|/Game/Project/Player/BluePrints/BP_FirstPersonCharacter.BP_FirstPersonCharacter_C|GetFirstPersonCamera _asbp_first_person_character))
  ;[0.15 0.15 0.15 0.5] 榴弾
  (Game|SpawnActorfromClass "/Game/Project/Player/BluePrints/BP_Skill_Grenade.BP_Skill_Grenade_C" (Math|Transform|MakeTransform (Transformation|GetWorldLocation _firstpersoncamera) (Transformation|GetWorldRotation _firstpersoncamera)) "AdjustIfPossibleButAlwaysSpawn" "MultiplyWithRoot" 0 0))

(event Custom|UseSkill
  (params (SkillID :type Integer))
  ;[0.15 0.15 0.15 0.5] 攻撃スキルの呼び出し
  (switch int SkillID
    (:201
      (CallFunction|Blade))
    (:202
      (CallFunction|Beam))
    (:203
      (CallFunction|Mine))
    (:204
      (CallFunction|Turret))
    (:205
      (CallFunction|Grenade))))

(event Custom|Mine
  (bind _returnvalue (Game|GetPlayerCharacter 0))
  (bind _asbp_first_person_character (Utilities|Casting|CastToBP_FirstPersonCharacter _returnvalue))
  (bind _firstpersoncamera (Variables|/Game/Project/Player/BluePrints/BP_FirstPersonCharacter.BP_FirstPersonCharacter_C|GetFirstPersonCamera _asbp_first_person_character))
  ;[0.15 0.15 0.15 0.5] 地雷
  (bind _outhit (Collision|LineTraceByChannel (Transformation|GetWorldLocation _firstpersoncamera) (+ (Transformation|GetWorldLocation _firstpersoncamera) (* (Math|Vector|GetForwardVector _firstpersoncamera) 5e+03)) "TraceTypeQuery1" true 0 "None"))
  (Game|SpawnActorfromClass "/Game/Project/Player/BluePrints/BP_SkillMine.BP_SkillMine_C" (Math|Transform|MakeTransform (.Location (Collision|BreakHitResult _outhit))) "Undefined" "MultiplyWithRoot" 0 0))

(event Custom|StartBeam
  ;[0.15 0.15 0.15 0.5] ビーム
  (Utilities|Time|SetTimerbyEvent (delegate Custom|Beam) 0.016 true))

(fn ConstructionScript)