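; Base enemy for a game where enemies slide along world X at the player's speed minus their own.
; Once no longer ahead of the player, it deals damage once and destroys itself.
; Lethal damage disables collision and calls the empty DieAnim hook.
; A separate Die event, not called here, applies life drain, rolls chest, fuel or heal drops written straight into player status, and increments the kill count.
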(event Custom|Die
  (bind _returnvalue (Game|GetPlayerCharacter 0))
  (bind _asbp_first_person_character (Utilities|Casting|CastToBP_FirstPersonCharacter _returnvalue))
  (bind _playerstatus (Variables|/Game/Project/Player/BluePrints/BP_FirstPersonCharacter.BP_FirstPersonCharacter_C|GetPlayerStatus _asbp_first_person_character))
  ;[0.15 0.15 0.15 0.5] ドロップアイテム
  (CallFunction|PlayerVamp)
  (Variables|Default|SetDropRoll (Math|Random|RandomFloatinRange 0.0 1e+02))
  (if (<= (Variables|Default|GetDropRoll) 5.0)
    (CallFunction|DropChest)
    (elif (<= (Variables|Default|GetDropRoll) 1e+01)
      (CallFunction|DropFuelItem)
      (elif (<= (Variables|Default|GetDropRoll) 15.0)
        (CallFunction|DropHealItem))))
  (Utilities|Struct|SetmembersinS_PlayerStatus _playerstatus (+ (.KillCount (Utilities|Struct|BreakS_PlayerStatus _playerstatus)) 1))
  (CallFunction|DieWait))

(event Custom|DieAnim)

(event Custom|DieWait
  (Collision|SetCollisionEnabled (Variables|Default|GetSkeletalMesh) "NoCollision")
  (CallFunction|DieAnim))

(event Game|Damage|EventAnyDamage
  (params (Damage :type Float%20%28single-precision%29) (DamageType :type Damage%20Type%20Object%20Reference) (InstigatedBy :type Controller%20Object%20Reference) (DamageCauser :type Actor%20Object%20Reference))
  (bind _isdie (CallFunction|IsDie))
  (if (not _isdie)
    (CallFunction|TakeDamage Damage)
    (bind _isdie_2 (CallFunction|IsDie))
    (if _isdie_2
      (Collision|SetCollisionEnabled (Variables|Default|GetSkeletalMesh) "NoCollision")
      (CallFunction|DieAnim))))

(event EventTick
  (params (DeltaSeconds :type Float%20%28single-precision%29))
  ;[0.15 0.15 0.15 0.5] Update
  (bind _bool (CallFunction|IsEnemyinFront))
  (if _bool
    (CallFunction|Move DeltaSeconds)
    (else
      (CallFunction|AttacktoPlayer))))

(fn ConstructionScript)

(fn DropChest
  (bind _returnvalue (Game|GetPlayerCharacter 0))
  (bind _asbp_first_person_character (Utilities|Casting|CastToBP_FirstPersonCharacter _returnvalue))
  (bind _playerstatus (Variables|/Game/Project/Player/BluePrints/BP_FirstPersonCharacter.BP_FirstPersonCharacter_C|GetPlayerStatus _asbp_first_person_character))
  ;[0.15 0.15 0.15 0.5] 宝箱ドロップ
  (Utilities|Struct|SetmembersinS_PlayerStatus _playerstatus (+ (.ChestCount (Utilities|Struct|BreakS_PlayerStatus _playerstatus)) 1.0))
  (Development|PrintString "宝箱獲得")
  (Audio|PlaySound2D "/Game/Project/Player/Assets/SE/drop.drop" 1.0 1.0 0.0 0 0))

(fn DropFuelItem
  (bind _returnvalue (Game|GetPlayerCharacter 0))
  (bind _asbp_first_person_character (Utilities|Casting|CastToBP_FirstPersonCharacter _returnvalue))
  (bind _playerstatus (Variables|/Game/Project/Player/BluePrints/BP_FirstPersonCharacter.BP_FirstPersonCharacter_C|GetPlayerStatus _asbp_first_person_character))
  (bind _fuel (Utilities|Struct|BreakS_PlayerStatus _playerstatus))
  (bind _returnvalue_2 (+ _fuel 3e+01))
  ;[0.15 0.15 0.15 0.5] 燃料回復アイテムドロップ
  (Utilities|Struct|SetmembersinS_PlayerStatus _playerstatus _returnvalue_2 _returnvalue_2)
  (Development|PrintString "燃料回復アイテム")
  (Audio|PlaySound2D "/Game/Project/Player/Assets/SE/jump.jump" 1.0 1.0 0.0 0 0))

(fn DropHealItem
  (bind _returnvalue (Game|GetPlayerCharacter 0))
  (bind _asbp_first_person_character (Utilities|Casting|CastToBP_FirstPersonCharacter _returnvalue))
  (bind _playerstatus (Variables|/Game/Project/Player/BluePrints/BP_FirstPersonCharacter.BP_FirstPersonCharacter_C|GetPlayerStatus _asbp_first_person_character))
  (bind _hp (Utilities|Struct|BreakS_PlayerStatus _playerstatus))
  (bind _returnvalue_2 (+ _hp 3e+01))
  ;[0.15 0.15 0.15 0.5] ＨＰ回復アイテム
  (Utilities|Struct|SetmembersinS_PlayerStatus _playerstatus _returnvalue_2 _returnvalue_2)
  (Development|PrintString "ＨＰ回復アイテム")
  (Audio|PlaySound2D "/Game/Project/Player/Assets/SE/jump.jump" 1.0 1.0 0.0 0 0))

(fn Move
  (params (GetDeltaTime :type Float%20%28double-precision%29))
  ;[0.15 0.15 0.15 0.5] 敵の移動処理
  (Transformation|AddActorWorldOffset (Math|Vector|MakeVector (* GetDeltaTime (- (.MoveSpeed (Utilities|Struct|BreakS_PlayerStatus (Variables|/Game/Project/Player/BluePrints/BP_FirstPersonCharacter.BP_FirstPersonCharacter_C|GetPlayerStatus (.AsBP%20First%20Person%20Character (Utilities|Casting|CastToBP_FirstPersonCharacter (Game|GetPlayerCharacter 0)))))) (.MoveSpeed (Utilities|Struct|BreakS_EnemyStatus (Variables|Default|GetEnemyStatus))))) 0.0 0.0)))

(fn IsEnemyinFront
  ;[0.15 0.15 0.15 0.5] エネミーがプレイヤーより手前かどうか
  (return (< (.x (Transformation|GetActorLocation (Game|GetPlayerCharacter 0))) (.x (Transformation|GetActorLocation)))))

(fn AttacktoPlayer
  ;[0.15 0.15 0.15 0.5] プレイヤーへのダメージ処理
  (bind _asbp_first_person_character (Utilities|Casting|CastToBP_FirstPersonCharacter (Game|GetPlayerCharacter 0)))
  (Default|TakeDamage _asbp_first_person_character (.Attack (Utilities|Struct|BreakS_EnemyStatus (Variables|Default|GetEnemyStatus))))
  (Actor|DestroyActor :!pinned true) ; プレイヤーの後ろに行ったときにダメージは一回だけしか入ってほしくないのですぐに削除
)

(fn TakeDamage
  (params (Damage :type Float%20%28double-precision%29))
  ;[0.15 0.15 0.15 0.5] エネミーのＨＰ減らす処理
  (Variables|Default|SetEnemyStatus (Utilities|Struct|MakeS_EnemyStatus (.MaxHP (Utilities|Struct|BreakS_EnemyStatus (Variables|Default|GetEnemyStatus))) (- (.HP (Utilities|Struct|BreakS_EnemyStatus (Variables|Default|GetEnemyStatus))) Damage) (.Attack (Utilities|Struct|BreakS_EnemyStatus (Variables|Default|GetEnemyStatus))) (.Defense (Utilities|Struct|BreakS_EnemyStatus (Variables|Default|GetEnemyStatus))) (.MoveSpeed (Utilities|Struct|BreakS_EnemyStatus (Variables|Default|GetEnemyStatus))))))

(fn IsDie
  ;[0.15 0.15 0.15 0.5] 死亡判定
  (if (>= (.HP (Utilities|Struct|BreakS_EnemyStatus (Variables|Default|GetEnemyStatus))) 0.1)
    (return false)
    (else
      (return true))))

(fn SetHP
  (params (HP :type Integer))
  ;[0.15 0.15 0.15 0.5] 敵のＨＰの増加
  (Variables|Default|SetEnemyStatus (Utilities|Struct|MakeS_EnemyStatus (.MaxHP (Utilities|Struct|BreakS_EnemyStatus (Variables|Default|GetEnemyStatus))) (+ HP (.HP (Utilities|Struct|BreakS_EnemyStatus (Variables|Default|GetEnemyStatus)))) (.Attack (Utilities|Struct|BreakS_EnemyStatus (Variables|Default|GetEnemyStatus))) (.Defense (Utilities|Struct|BreakS_EnemyStatus (Variables|Default|GetEnemyStatus))) (.MoveSpeed (Utilities|Struct|BreakS_EnemyStatus (Variables|Default|GetEnemyStatus))))))

(fn PlayerVamp
  (bind _returnvalue (Game|GetPlayerCharacter 0))
  (bind _asbp_first_person_character (Utilities|Casting|CastToBP_FirstPersonCharacter _returnvalue))
  (bind _playerstatus (Variables|/Game/Project/Player/BluePrints/BP_FirstPersonCharacter.BP_FirstPersonCharacter_C|GetPlayerStatus _asbp_first_person_character))
  (bind (_maxhp _hp _maxfuel _fuel _attack _attackspeed _defense _movespeed _regen _drain) (Utilities|Struct|BreakS_PlayerStatus _playerstatus))
  ;[0.15 0.15 0.15 0.5] プレイヤー側処理：体力吸収
  (Utilities|Struct|SetmembersinS_PlayerStatus _playerstatus (+ _hp _drain) 0.0))