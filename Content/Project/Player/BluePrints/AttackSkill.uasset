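; AttackSkill is a Blueprint holding the player's attack skills as events, with damage scaled from the first-person character's Attack status.
; Blade deals full radial damage around the player, ignoring the player, and draws a debug sphere.
; Beam multi-line traces forward from the camera on the Visibility channel and damages each returned hit, with debug drawing.
; UseSkill, Mine, Turret and Grenade are empty stubs.
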(event Custom|Blade
  (bind _returnvalue (Game|GetPlayerCharacter 0))
  (bind _asbp_first_person_character (Utilities|Casting|CastToBP_FirstPersonCharacter _returnvalue))
  (bind _returnvalue_2 (Transformation|GetActorLocation _asbp_first_person_character))
  ;[0.15 0.15 0.15 0.5] ブレード
  (Game|Damage|ApplyRadialDamage (* (.Attack (Utilities|Struct|BreakS_PlayerStatus (Variables|/Game/Project/Player/BluePrints/BP_FirstPersonCharacter.BP_FirstPersonCharacter_C|GetPlayerStatus _asbp_first_person_character))) 3.0) _returnvalue_2 1e+03 0 (Utilities|Array|MakeArray _asbp_first_person_character) 0 0 true "ECC_Visibility")
  (Rendering|Debug|DrawDebugSphere _returnvalue_2 1e+03 12 "(R=1.000000,G=1.000000,B=1.000000,A=1.000000)" 1.0))

(event Custom|Beam
  (bind _returnvalue (Game|GetPlayerCharacter 0))
  (bind _asbp_first_person_character (Utilities|Casting|CastToBP_FirstPersonCharacter _returnvalue))
  (bind _firstpersoncamera (Variables|/Game/Project/Player/BluePrints/BP_FirstPersonCharacter.BP_FirstPersonCharacter_C|GetFirstPersonCamera _asbp_first_person_character))
  (bind _returnvalue_2 (Transformation|GetWorldLocation _firstpersoncamera))
  ;[0.15 0.15 0.15 0.5] ビーム
  (bind _outhits (Collision|MultiLineTraceByChannel _returnvalue_2 (+ _returnvalue_2 (* (Math|Vector|GetForwardVector _firstpersoncamera) 1e+04)) "TraceTypeQuery1" false 0 "ForDuration"))
  (for _array_element _outhits
    (Game|Damage|ApplyDamage (.HitActor (Collision|BreakHitResult _array_element)) (* (.Attack (Utilities|Struct|BreakS_PlayerStatus (Variables|/Game/Project/Player/BluePrints/BP_FirstPersonCharacter.BP_FirstPersonCharacter_C|GetPlayerStatus (.AsBP%20First%20Person%20Character (Utilities|Casting|CastToBP_FirstPersonCharacter (Game|GetPlayerCharacter 0)))))) 2.5) 0 0)))

(event Custom|CustomEvent)

(event Custom|Turret)

(event Custom|Grenade)

(event Custom|UseSkill
  (params (SkillID :type Integer)))

(event Custom|Mine)

(fn ConstructionScript)