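; BP_SkillMine is a player skill mine that explodes when an enemy touches it.
; An overlap on its Sphere by a BP_EnemyBase applies full, falloff-free radial damage scaled from the first-person player's Attack stat.
; It then spawns the NS_Explosion effect and destroys itself.
; A debug sphere is also drawn at detonation, with a smaller radius than the actual damage area.
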(event OnComponentBeginOverlap(Sphere)
  (params (OverlappedComponent :type Primitive%20Component%20Object%20Reference) (OtherActor :type Actor%20Object%20Reference) (OtherComp :type Primitive%20Component%20Object%20Reference) (OtherBodyIndex :type Integer) (bFromSweep :type Boolean) (SweepResult :type Hit%20Result%20Structure%20%28by%20ref%29))
  (bind _returnvalue (Transformation|GetActorLocation))
  (Utilities|Casting|CastToBP_EnemyBase OtherActor)
  (Game|Damage|ApplyRadialDamage (* (.Attack (Utilities|Struct|BreakS_PlayerStatus (Variables|/Game/Project/Player/BluePrints/BP_FirstPersonCharacter.BP_FirstPersonCharacter_C|GetPlayerStatus (.AsBP%20First%20Person%20Character (Utilities|Casting|CastToBP_FirstPersonCharacter (Game|GetPlayerCharacter 0)))))) 4.0) _returnvalue 7e+02 0 0 0 0 true "ECC_Visibility")
  (Niagara|SpawnSystematLocation "/Game/NiagaraExamples/FX_Explosions/NS_Explosion.NS_Explosion" _returnvalue)
  (Rendering|Debug|DrawDebugSphere _returnvalue 5e+02 12 "(R=1.000000,G=0.000509,B=0.000000,A=1.000000)" 1.0)
  (Actor|DestroyActor))

(fn ConstructionScript)