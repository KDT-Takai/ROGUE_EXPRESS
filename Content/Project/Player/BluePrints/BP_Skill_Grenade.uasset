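; BP_Skill_Grenade is a player skill grenade actor that explodes when its static mesh hits something.
; On hit it applies full, non-falloff radial damage around a slightly raised origin, scaled from the Attack in the first-person character's PlayerStatus.
; It then spawns a Niagara explosion, draws a debug sphere of the blast radius, plays a sound and destroys itself.
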(event OnComponentHit(StaticMesh)
  (params (HitComponent :type Primitive%20Component%20Object%20Reference) (OtherActor :type Actor%20Object%20Reference) (OtherComp :type Primitive%20Component%20Object%20Reference) (NormalImpulse :type Vector :default "0, 0, 0") (Hit :type Hit%20Result%20Structure%20%28by%20ref%29))
  (bind _returnvalue (Transformation|GetActorLocation))
  (bind _returnvalue_2 (+ _returnvalue "0.000000,0.000000,30.000000"))
  (Game|Damage|ApplyRadialDamage (* (.Attack (Utilities|Struct|BreakS_PlayerStatus (Variables|/Game/Project/Player/BluePrints/BP_FirstPersonCharacter.BP_FirstPersonCharacter_C|GetPlayerStatus (.AsBP%20First%20Person%20Character (Utilities|Casting|CastToBP_FirstPersonCharacter (Game|GetPlayerCharacter 0)))))) 4.0) _returnvalue_2 6e+02 0 0 0 0 true "ECC_Visibility")
  (Niagara|SpawnSystematLocation "/Game/NiagaraExamples/FX_Explosions/NS_Explosion.NS_Explosion" _returnvalue_2)
  (Rendering|Debug|DrawDebugSphere _returnvalue_2 6e+02 12 "(R=1.000000,G=0.000000,B=0.000000,A=1.000000)" 1.0)
  (Audio|PlaySoundatLocation "/Game/Project/Player/Assets/SE/Explosion04-1_Short_.Explosion04-1_Short_" (Transformation|GetActorLocation) "0, 0, 0" 1.0 1.0 0.0 0 0 0 0)
  (Actor|DestroyActor))

(fn ConstructionScript)