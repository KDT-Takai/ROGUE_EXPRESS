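; BP_WaveManager runs a timed enemy wave and hands off to the result level when it ends.
; A looping timer spawns random batches of drones and ground-level buggies ahead of the player along world +X.
; Batch size scales with the GameInstance's current wave, which also sets the HP value passed to each enemy.
; After 60 seconds counted on Tick, it stops spawning, records player status in the GameInstance and opens Lvl_Result.
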(event Custom|SpawnEnemyEvent
  ;[0.15 0.15 0.15 0.5] Update
  ;;[0.15 0.15 0.15 0.5] 敵の生成処理
  (CallFunction|SpownEnemy))

(event EventBeginPlay
  ;[0.15 0.15 0.15 0.5] Update
  (bind _returnvalue (Utilities|Time|SetTimerbyEvent (delegate Custom|SpawnEnemyEvent) (Variables|Default|GetSpawnInterval) true))
  (bind _output_get (Variables|Default|SetSpawnTimerHandle _returnvalue)))

(event EventTick
  (params (DeltaSeconds :type Float%20%28single-precision%29))
  ;[0.15 0.15 0.15 0.5] Update
  (CallFunction|WaveCount DeltaSeconds)
  (if (>= (Variables|Default|GetWaveTime) 6e+01)
    (Utilities|FlowControl|DoOnce false
      (:Completed
        (Utilities|Time|ClearandInvalidateTimerbyHandle (stale EventBeginPlay _output_get))
        (CallFunction|SaveandGoNextLevel)))))

(fn ConstructionScript)

(fn SpownEnemy
  (bind _returnvalue (Game|GetGameInstance))
  (bind _returnvalue_2 (Game|GetPlayerCharacter 0))
  (bind _returnvalue_3 (Transformation|GetActorLocation _returnvalue_2))
  (bind _asbp_game_instance (Utilities|Casting|CastToBP_GameInstance _returnvalue))
  (bind _currentwave (Variables|/Game/Project/System/BP_GameInstance.BP_GameInstance_C|GetCurrentWave _asbp_game_instance))
  ;[0.15 0.15 0.15 0.5] 敵の生成処理
  (switch int (Math|Random|RandomIntegerinRange 0 2)
    (:0
      (for _index (range 1 (* _currentwave 3))
        (Variables|Default|SetSpawnChara (Math|Random|RandomBool))
        (bind _returnvalue_4 (Game|SpawnActorfromClass (select (Variables|Default|GetSpawnChara) "/Game/Project/Player/BluePrints/BP_Drone.BP_Drone_C" "/Game/Project/Player/BluePrints/BP_Buggy.BP_Buggy_C") (Math|Transform|MakeTransform (Math|Vector|MakeVector (+ (.x _returnvalue_3) (Math|Random|RandomFloatinRange 6e+03 6.2e+03)) (+ (.y _returnvalue_3) (Math|Random|RandomFloatinRange -1.5e+03 1.5e+03)) (Math|Float|SelectFloat (+ (.z _returnvalue_3) (Math|Random|RandomFloatinRange 8e+01 8e+02)) 0.0 (Variables|Default|GetSpawnChara))) "0, 0, 0" "1.000000,1.000000,1.000000") "Undefined" "MultiplyWithRoot" 0 0))
        ;[0.15 0.15 0.15 0.5] ウェーブごとにＨＰ25増加させる
        (bind _asbp_enemy_base (Utilities|Casting|CastToBP_EnemyBase _returnvalue_4))
        (Default|SetHP _asbp_enemy_base (* (- (Variables|/Game/Project/System/BP_GameInstance.BP_GameInstance_C|GetCurrentWave (.AsBP%20Game%20Instance (Utilities|Casting|CastToBP_GameInstance (Game|GetGameInstance)))) 1) 25))))
    (:1
      (for _index_2 (range 1 (* _currentwave 5))
        (Variables|Default|SetSpawnChara (Math|Random|RandomBool))
        (bind _returnvalue_5 (Game|SpawnActorfromClass (select (Variables|Default|GetSpawnChara) "/Game/Project/Player/BluePrints/BP_Drone.BP_Drone_C" "/Game/Project/Player/BluePrints/BP_Buggy.BP_Buggy_C") (Math|Transform|MakeTransform (Math|Vector|MakeVector (+ (.x _returnvalue_3) (Math|Random|RandomFloatinRange 6e+03 6.2e+03)) (+ (.y _returnvalue_3) (Math|Random|RandomFloatinRange -1.5e+03 1.5e+03)) (Math|Float|SelectFloat (+ (.z _returnvalue_3) (Math|Random|RandomFloatinRange 8e+01 8e+02)) 0.0 (Variables|Default|GetSpawnChara))) "0, 0, 0" "1.000000,1.000000,1.000000") "Undefined" "MultiplyWithRoot" 0 0))
        (bind _asbp_enemy_base_2 (Utilities|Casting|CastToBP_EnemyBase _returnvalue_5))
        (Default|SetHP _asbp_enemy_base_2 (* (- (Variables|/Game/Project/System/BP_GameInstance.BP_GameInstance_C|GetCurrentWave (.AsBP%20Game%20Instance (Utilities|Casting|CastToBP_GameInstance (Game|GetGameInstance)))) 1) 25))))
    (:2
      (for _index_3 (range 1 (* _currentwave 10))
        (Variables|Default|SetSpawnChara (Math|Random|RandomBool))
        (bind _returnvalue_6 (Game|SpawnActorfromClass (select (Variables|Default|GetSpawnChara) "/Game/Project/Player/BluePrints/BP_Drone.BP_Drone_C" "/Game/Project/Player/BluePrints/BP_Buggy.BP_Buggy_C") (Math|Transform|MakeTransform (Math|Vector|MakeVector (+ (.x _returnvalue_3) (Math|Random|RandomFloatinRange 6e+03 6.2e+03)) (+ (.y _returnvalue_3) (Math|Random|RandomFloatinRange -1.5e+03 1.5e+03)) (Math|Float|SelectFloat (+ (.z _returnvalue_3) (Math|Random|RandomFloatinRange 8e+01 8e+02)) 0.0 (Variables|Default|GetSpawnChara))) "0, 0, 0" "1.000000,1.000000,1.000000") "Undefined" "MultiplyWithRoot" 0 0))
        (bind _asbp_enemy_base_3 (Utilities|Casting|CastToBP_EnemyBase _returnvalue_6))
        (Default|SetHP _asbp_enemy_base_3 (* (- (Variables|/Game/Project/System/BP_GameInstance.BP_GameInstance_C|GetCurrentWave (.AsBP%20Game%20Instance (Utilities|Casting|CastToBP_GameInstance (Game|GetGameInstance)))) 1) 25))))))

(fn WaveCount
  (params (GetDeltaTime :type Float%20%28double-precision%29))
  ;[0.15 0.15 0.15 0.5] ウェーブ時間のカウント追加
  (bind _output_get (Variables|Default|SetWaveTime (+ GetDeltaTime (Variables|Default|GetWaveTime))))
  (Development|PrintString (Utilities|String|ToString(Text) (Utilities|Text|FormatText "WaveTime:{WaveTime}" _output_get)) true true "(R=0.000000,G=0.660000,B=1.000000,A=1.000000)" 0.0))

(fn SaveandGoNextLevel
  ;[0.15 0.15 0.15 0.5] 保存処理を行ってからリザルトへ移行
  (bind _asbp_game_instance (Utilities|Casting|CastToBP_GameInstance (Game|GetGameInstance)))
  (bind _asbp_first_person_character (Utilities|Casting|CastToBP_FirstPersonCharacter (Game|GetPlayerCharacter 0)))
  (Default|RecordWaveResult _asbp_game_instance (Variables|/Game/Project/Player/BluePrints/BP_FirstPersonCharacter.BP_FirstPersonCharacter_C|GetPlayerStatus _asbp_first_person_character))
  (Development|PrintString "ここでリザルト画面へ移行させる")
  (Game|OpenLevel(byName) "Lvl_Result"))