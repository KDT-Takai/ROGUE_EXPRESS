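; BP_Bullet is a player projectile that damages enemies.
; Each Tick it moves along its right vector at Speed with a swept offset, and it expires after a short lifespan set on BeginPlay.
; When its Box overlaps a living BP_EnemyBase, it applies Damage, calls Die on the enemy if that kills it, and destroys itself.
; Other actors and already-dead enemies are ignored by the overlap handler.
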(event OnComponentBeginOverlap(Box)
  (params (OverlappedComponent :type Primitive%20Component%20Object%20Reference) (OtherActor :type Actor%20Object%20Reference) (OtherComp :type Primitive%20Component%20Object%20Reference) (OtherBodyIndex :type Integer) (bFromSweep :type Boolean) (SweepResult :type Hit%20Result%20Structure%20%28by%20ref%29))
  ;[0.15 0.15 0.15 0.5] 弾と敵の衝突判定とダメージ処理
  (bind _asbp_enemy_base (Utilities|Casting|CastToBP_EnemyBase OtherActor))
  (bind _isdie (Default|IsDie _asbp_enemy_base))
  (if (not _isdie)
    (Default|TakeDamage _asbp_enemy_base (Variables|Default|GetDamage))
    (bind _isdie_2 (Default|IsDie _asbp_enemy_base))
    (if _isdie_2
      (Default|Die _asbp_enemy_base)
      (Actor|DestroyActor)
      (else
        (Actor|DestroyActor)))))

(event EventBeginPlay
  ;[0.15 0.15 0.15 0.5] 寿命設定
  (Actor|SetLifeSpan 3.0))

(event EventTick
  (params (DeltaSeconds :type Float%20%28single-precision%29))
  ;[0.15 0.15 0.15 0.5] 弾を飛ばす処理
  (Transformation|AddActorWorldOffset (* DeltaSeconds (Transformation|GetActorRightVector) (Variables|Default|GetSpeed)) true))

(fn ConstructionScript)