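; BP_MG is the player's machine gun actor, which follows the first-person view and fires bullets.
; InitializeGun, called by the player at game start, attaches the gun to the camera and sets its offset and scale.
; Tick maps camera pitch and yaw to gun rotation, capping downward tilt to prevent ground clipping.
; PlayShootEffect spawns a muzzle flash, a BP_Bullet carrying the given damage, and a gunshot sound at the muzzle socket.
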(event EventTick
  (params (DeltaSeconds :type Float%20%28single-precision%29))
  (bind _returnvalue (Game|GetPlayerCharacter 0))
  (bind _asbp_first_person_character (Utilities|Casting|CastToBP_FirstPersonCharacter _returnvalue))
  (bind _firstpersoncamera (Variables|/Game/Project/Player/BluePrints/BP_FirstPersonCharacter.BP_FirstPersonCharacter_C|GetFirstPersonCamera _asbp_first_person_character))
  (bind _returnvalue_2 (Transformation|GetWorldRotation _firstpersoncamera))
  (bind _returnvalue_3 (- (.yaw _returnvalue_2) 9e+01))
  (bind _returnvalue_4 (* (.pitch _returnvalue_2) -1.0))
  ;[0.15 0.15 0.15 0.5] プレイヤーの視点に合わせてマシンガンの回転
  (if (< _returnvalue_4 9.0)
    (Transformation|SetActorRotation (Math|Rotator|MakeRotator _returnvalue_4 0.0 _returnvalue_3))
    (else
      (Transformation|SetActorRotation (Math|Rotator|MakeRotator 9.0 0.0 _returnvalue_3)) ; ９以上の場合地面にめり込むため、上限値を設定
    )))

(fn ConstructionScript)

(fn InitializeGun
  ;[0.15 0.15 0.15 0.5] 銃の初期化処理　ゲーム開始時にプレイヤー側で呼ぶ
  (Transformation|AttachComponentToComponent (Variables|Default|GetGunRef) (Variables|/Game/Project/Player/BluePrints/BP_FirstPersonCharacter.BP_FirstPersonCharacter_C|GetFirstPersonCamera (.AsBP%20First%20Person%20Character (Utilities|Casting|CastToBP_FirstPersonCharacter (Game|GetPlayerCharacter 0)))) "None" "KeepRelative" "SnapToTarget" "KeepWorld" true)
  (Transformation|SetActorRelativeLocation "61.000000,0.000000,90.000000")
  (Transformation|SetActorRelativeScale3D "15.580000,15.580000,15.580000"))

(fn PlayShootEffect
  (params (Damage :type Float%20%28double-precision%29))
  (bind _mg (Variables|Default|GetMG))
  (bind _returnvalue (Transformation|GetSocketLocation _mg "MuzzleSocket"))
  ;[0.15 0.15 0.15 0.5] 弾の表示
  (Niagara|SpawnSystemAttached "/Game/NiagaraExamples/FX_Weapons/MuzzleFlashes/NS_MuzzleFlash.NS_MuzzleFlash" _mg "MuzzleSocket" "0, 0, 0" "0.000000,90.000000,0.000000" "SnapToTarget" true)
  (bind _returnvalue_2 (Game|SpawnActorfromClass "/Game/Project/Player/BluePrints/BP_Bullet.BP_Bullet_C" (Math|Transform|MakeTransform _returnvalue (Transformation|GetActorRotation) "1.000000,1.000000,1.000000") "AlwaysSpawn" "MultiplyWithRoot" 0 0))
  (Variables|/Game/Project/Player/BluePrints/BP_Bullet.BP_Bullet_C|SetDamage _returnvalue_2 Damage)
  (Audio|PlaySoundatLocation "/Game/Project/Player/Assets/SE/Gunshot01-1.Gunshot01-1" _returnvalue "0, 0, 0" 1.0 1.0 0.0 0 0 0 0))