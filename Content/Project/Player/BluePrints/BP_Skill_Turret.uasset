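; BP_Skill_Turret is a turret skill actor that automatically damages nearby enemies.
; A looping one-second timer started on BeginPlay fires at the first BP_EnemyBase overlapping its Sphere, skipping the shot if that enemy is dead.
; Hits apply instant damage equal to twice the player character's Attack stat, with a brief red debug line as the shot visual.
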(event Custom|Fire
  (bind _sphere (Variables|Default|GetSphere))
  (bind _overlappingactors (Collision|GetOverlappingActors _sphere "/Game/Project/Player/BluePrints/BP_EnemyBase.BP_EnemyBase_C" :!class /Script/Engine.PrimitiveComponent))
  (bind _output (Utilities|Array|Get(acopy) _overlappingactors))
  (Utilities|IsValid _output
    (:Is%20Valid
      (bind _isdie (Default|IsDie (.AsBP%20Enemy%20Base (Utilities|Casting|CastToBP_EnemyBase _output))))
      (if (not _isdie)
        (Game|Damage|ApplyDamage _output (* (.Attack (Utilities|Struct|BreakS_PlayerStatus (Variables|/Game/Project/Player/BluePrints/BP_FirstPersonCharacter.BP_FirstPersonCharacter_C|GetPlayerStatus (.AsBP%20First%20Person%20Character (Utilities|Casting|CastToBP_FirstPersonCharacter (Game|GetPlayerCharacter 0)))))) 2.0) 0 0)
        (Rendering|Debug|DrawDebugLine (Transformation|GetActorLocation) (Transformation|GetActorLocation _output) "(R=1.000000,G=0.000000,B=0.000000,A=1.000000)" 0.1 0.0)))))

(event EventBeginPlay
  (Utilities|Time|SetTimerbyEvent (delegate Custom|Fire) 1.0 true))

(fn ConstructionScript)